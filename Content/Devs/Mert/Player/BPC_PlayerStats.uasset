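; Player stats component that tracks health and stamina and their maximums for the player character.
; On BeginPlay it caches the player character, whose HUD health bar is refreshed whenever health or max health changes.
; Decrease functions return true when the stat hits zero or below, while increase functions for current values cap at the maximum.
; Stamina has no HUD update, and the XP function is an empty stub.
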(event EventBeginPlay
  (bind _asbp_player_character (Utilities|Casting|CastToBP_Player_Character (Game|GetPlayerCharacter 0)))
  (Variables|Default|SetPlayer%20REF _asbp_player_character))

(event EventTick
  (params (DeltaSeconds :type Float%20%28single-precision%29)))

(fn DecreaseHealth
  (params (Damage%20Received :type Float%20%28double-precision%29))
  (bind _output_get (Variables|Health|SetHealth (- (Variables|Health|GetHealth) Damage%20Received)))
  (Progress|SetPercent (Variables|/Game/Devs/Mert/Player/UI/Player_HUD_W.Player_HUD_W_C|GetHealthBar (Variables|/Game/SurvivorsTemplate/Blueprints/Character/BP_Player_Character.BP_Player_Character_C|GetHUD%20REF (Variables|Default|GetPlayer%20REF))) (/ _output_get (Variables|Health|GetMax%20Health)))
  (if (<= _output_get 0.0)
    (return true)
    (else
      (return false))))

(fn IncreaseMaxHealth
  (params (Max%20Health%20Increase :type Float%20%28double-precision%29))
  (Variables|Health|SetMax%20Health (+ (Variables|Health|GetMax%20Health) Max%20Health%20Increase))
  (Progress|SetPercent (Variables|/Game/Devs/Mert/Player/UI/Player_HUD_W.Player_HUD_W_C|GetHealthBar (Variables|/Game/SurvivorsTemplate/Blueprints/Character/BP_Player_Character.BP_Player_Character_C|GetHUD%20REF (Variables|Default|GetPlayer%20REF))) (/ (Variables|Health|GetHealth) (Variables|Health|GetMax%20Health))))

(fn DecreaseStamina
  (params (Stamina%20Decrease :type Float%20%28double-precision%29))
  (bind _output_get (Variables|Stamina|SetStamina (- (Variables|Stamina|GetStamina) Stamina%20Decrease)))
  (if (<= _output_get 0.0)
    (return true)
    (else
      (return false))))

(fn IncreaseMaxStamina
  (params (Max%20Stamina%20Increase :type Float%20%28double-precision%29))
  (Variables|Stamina|SetMax%20Stamina (+ (Variables|Stamina|GetMax%20Stamina) Max%20Stamina%20Increase)))

(fn IncreaseXP)

(fn IncreaseHealth
  (params (Health%20Increase :type Float%20%28double-precision%29))
  (bind _output_get (Variables|Health|SetHealth (+ (Variables|Health|GetHealth) Health%20Increase)))
  (if (> _output_get (Variables|Health|GetMax%20Health))
    (bind _output_get_2 (Variables|Health|SetHealth (Variables|Health|GetMax%20Health))))
  (Progress|SetPercent (Variables|/Game/Devs/Mert/Player/UI/Player_HUD_W.Player_HUD_W_C|GetHealthBar (Variables|/Game/SurvivorsTemplate/Blueprints/Character/BP_Player_Character.BP_Player_Character_C|GetHUD%20REF (Variables|Default|GetPlayer%20REF))) (/ _output_get_2 (Variables|Health|GetMax%20Health))))

(fn IncreaseStamina
  (params (Stamina%20Increase :type Float%20%28double-precision%29))
  (bind _output_get (Variables|Stamina|SetStamina (+ (Variables|Stamina|GetStamina) Stamina%20Increase)))
  (if (> _output_get (Variables|Stamina|GetMax%20Stamina))
    (Variables|Stamina|SetStamina (Variables|Stamina|GetMax%20Stamina))))