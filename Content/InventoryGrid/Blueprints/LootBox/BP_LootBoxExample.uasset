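; Example interactable loot box with a randomized mesh, a name widget and its own grid inventory component.
; On BeginPlay it fills with either manually selected items or random DT_ItemList rows filtered by item type, with randomized counts.
; Each item spawns as a temporary BP_BaseItemInventory actor, destroyed once added to the inventory.
; Interaction toggles the player's inventory UI in LootBox mode and binds the box's inventory to its grid panel.
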(event Custom|ExitLootBox
  ;[0 0.5 0.01618] OpenUI
  (Default|ToggleInventory (Variables|Default|GetInventory%20Component%20Player))
  (Variables|Components|SetOpen? false))

(event EventBeginPlay
  ;[0 0.5 0.01618] begin Play
  (Utilities|FlowControl|Sequence
    (:then_0
      (CallFunction|StaticMeshRandom)
      (CallFunction|GetAllItens)
      ;[1 0 0] Random
      (if (Variables|ConfigLootBox|GetRandomSpawn?)
        (CallFunction|RandomSpawn)
        (else
          (for _array_element (Variables|ConfigLootBox|GetSelect%20Manual%20ItensSpawnToLootBox)
            (CallFunction|AddItensLootBox _array_element)))))
    (:then_1
      (bind _aswb_name_item (Utilities|Casting|CastToWB_NameItem (UserInterface|GetUserWidgetObject (Variables|Default|GetWidget))))
      (bind _output_get (Variables|Default|SetAs%20WB%20Name%20Item _aswb_name_item))
      (Variables|/Game/InventoryGrid/Blueprints/Widget/WB_NameItem.WB_NameItem_C|SetNameItem _output_get (Utilities|String|ToString(Text) (Variables|ConfigLootBox|GetName))))))

(event EventStartInteraction
  (params (InventoryComponent :type BP%20Inventory%20Grid%20Component%20Object%20Reference))
  ;[0 0.5 0.01618] OpenUI
  (bind _output_get (Variables|Default|SetInventory%20Component%20Player InventoryComponent))
  (Variables|Components|SetOpen? (Widget|IsVisible (Variables|/Game/InventoryGrid/Blueprints/Modify_inventory/BP_InventoryGridComponent.BP_InventoryGridComponent_C|GetInventoryUI _output_get)))
  (if (Variables|Components|GetOpen?)
    (Default|ToggleInventory (Variables|Default|GetInventory%20Component%20Player))
    (Variables|Components|SetOpen? false)
    (else
      (Default|ToggleInventory (Variables|Default|GetInventory%20Component%20Player) "LootBox")
      (CallFunction|CheckComponents (Variables|/Game/InventoryGrid/Blueprints/Modify_inventory/BP_InventoryGridComponent.BP_InventoryGridComponent_C|GetInventoryUI (Variables|Default|GetInventory%20Component%20Player)))
      (Variables|Components|SetOpen? true))))

(event EventShowNameItem
  (params (Show? :type Boolean))
  ;[0 0.5 0.01618] begin Play
  (Rendering|SetVisibility (Variables|Default|GetWidget) Show? false))

(fn ConstructionScript
  (bind _static_mesh_variation (Variables|ConfigLootBox|GetStatic%20Mesh%20Variation))
  (bind _static_mesh_variation_2 (Variables|ConfigLootBox|GetStatic%20Mesh%20Variation))
  (bind _static_mesh_variation_3 (Variables|ConfigLootBox|GetStatic%20Mesh%20Variation))
  (bind _bp_inventorysystemcomponent (Variables|Default|GetBP_InventorySystemComponent))
  (bind _returnvalue (Utilities|Array|Length _static_mesh_variation_2))
  (bind _output (Utilities|Array|Get(acopy) _static_mesh_variation_3))
  (bind _returnvalue_2 (Math|Random|RandomInteger _returnvalue))
  (bind _output_2 (Utilities|Array|Get(acopy) _static_mesh_variation _returnvalue_2))
  (Variables|/Game/InventoryGrid/Blueprints/Modify_inventory/BP_InventoryGridComponent.BP_InventoryGridComponent_C|SetColumns _bp_inventorysystemcomponent (Variables|ConfigLootBox|GetColumns))
  (Variables|/Game/InventoryGrid/Blueprints/Modify_inventory/BP_InventoryGridComponent.BP_InventoryGridComponent_C|SetRows _bp_inventorysystemcomponent (Variables|ConfigLootBox|GetRows))
  (if (> (Utilities|Array|Length (Variables|ConfigLootBox|GetStatic%20Mesh%20Variation)) 0)
    (Utilities|IsValid _output_2
      (:Is%20Valid
        (Components|StaticMesh|SetStaticMesh (Variables|Default|GetStaticMesh) _output_2)))
    (else
      (Utilities|IsValid _output
        (:Is%20Valid
          (Components|StaticMesh|SetStaticMesh (Variables|Default|GetStaticMesh) _output))))))

(fn AddItensLootBox
  (params (ItemSelect :type S%20Item%20Select%20Structure))
  (bind _returnvalue (Game|SpawnActorfromClass "/Game/InventoryGrid/Blueprints/Modify_inventory/BP_BaseItemInventory.BP_BaseItemInventory_C" (Math|Transform|MakeTransform "0, 0, 0" "0, 0, 0" "1.000000,1.000000,1.000000") "Undefined" "OverrideRootScale" 0 0 ItemSelect 0 0))
  (bind _itemobject (Default|GetDefaultItemObject _returnvalue))
  (bind _success (Default|AddItemtoInventory (Variables|Default|GetBP_InventorySystemComponent) _itemobject false))
  (if _success
    (Actor|DestroyActor _returnvalue)))

(fn CheckComponents
  (params (InventoryUI :type WB%20Inventory%20Object%20Reference))
  (Utilities|IsValid (Variables|/Game/InventoryGrid/Blueprints/Modify_inventory/BP_InventoryGridComponent.BP_InventoryGridComponent_C|GetBackPack (Variables|Default|GetInventory%20Component%20Player))
    (:Is%20Valid
      (Default|GetInventorySettings (Variables|/Game/InventoryGrid/Blueprints/Widget/WB_LootBoxPanel.WB_LootBoxPanel_C|GetWB_GridPanelInventoryLootBox (Variables|/Game/InventoryGrid/Blueprints/Widget/WB_Inventory.WB_Inventory_C|GetWB_LootBox InventoryUI)) InventoryUI (Variables|Default|GetBP_InventorySystemComponent) (Variables|Default|GetInventory%20Component%20Player) 0 0 "" "NewEnumerator5" false))
    (:Is%20Not%20Valid
      (Default|GetInventorySettings (Variables|/Game/InventoryGrid/Blueprints/Widget/WB_LootBoxPanel.WB_LootBoxPanel_C|GetWB_GridPanelInventoryLootBox (Variables|/Game/InventoryGrid/Blueprints/Widget/WB_Inventory.WB_Inventory_C|GetWB_LootBox InventoryUI)) InventoryUI (Variables|Default|GetBP_InventorySystemComponent) (Variables|Default|GetInventory%20Component%20Player) 0 0 "" "NewEnumerator5" false)))
  (Default|Name (Variables|/Game/InventoryGrid/Blueprints/Widget/WB_Inventory.WB_Inventory_C|GetWB_LootBox (Variables|/Game/InventoryGrid/Blueprints/Modify_inventory/BP_InventoryGridComponent.BP_InventoryGridComponent_C|GetInventoryUI (Variables|Default|GetInventory%20Component%20Player))) (Variables|ConfigLootBox|GetName)))

(fn StaticMeshRandom
  (bind _static_mesh_variation (Variables|ConfigLootBox|GetStatic%20Mesh%20Variation))
  (bind _static_mesh_variation_2 (Variables|ConfigLootBox|GetStatic%20Mesh%20Variation))
  (bind _static_mesh_variation_3 (Variables|ConfigLootBox|GetStatic%20Mesh%20Variation))
  (bind _returnvalue (Utilities|Array|Length _static_mesh_variation_3))
  (bind _output (Utilities|Array|Get(acopy) _static_mesh_variation))
  (bind _returnvalue_2 (Math|Random|RandomInteger _returnvalue))
  (bind _output_2 (Utilities|Array|Get(acopy) _static_mesh_variation_2 _returnvalue_2))
  (if (> (Utilities|Array|Length (Variables|ConfigLootBox|GetStatic%20Mesh%20Variation)) 0)
    (Utilities|IsValid _output_2
      (:Is%20Valid
        (Components|StaticMesh|SetStaticMesh (Variables|Default|GetStaticMesh) _output_2)))
    (else
      (Utilities|IsValid _output
        (:Is%20Valid
          (Components|StaticMesh|SetStaticMesh (Variables|Default|GetStaticMesh) _output))))))

(fn RandomSpawn
  (bind _itensspawn (Variables|Default|GetItensSpawn))
  (for _array_element (Variables|ConfigLootBox|GetType%20Itens%20To%20Random%20Spawn)
    (for _array_element_2 (Variables|Default|GetAllItens)
      (bind _returnvalue (Utilities|GetDataTableRow (.DataTable (Utilities|Struct|BreakDataTableRowHandle (.ItemSelect (Utilities|Struct|BreakS_ItemSelect _array_element_2)))) (.RowName (Utilities|Struct|BreakDataTableRowHandle (.ItemSelect (Utilities|Struct|BreakS_ItemSelect _array_element_2)))))
        (:then
          (if (or (Utilities|Enum|Equal(Enum) (.TypeItem (Utilities|Struct|BreakS_ItemSettings _returnvalue)) (.TypeitensToSpawn (Utilities|Struct|BreakS_typeItensRandomSpawn _array_element))) (Utilities|Enum|Equal(Enum) (.TypeitensToSpawn (Utilities|Struct|BreakS_typeItensRandomSpawn _array_element)) "NewEnumerator6"))
            (Utilities|Array|Add (Variables|Default|GetItensSpawn) (Utilities|Struct|MakeS_ItemSelect (Utilities|Struct|MakeDataTableRowHandle "/Game/InventoryGrid/Blueprints/Modify_inventory/DT_ItemList.DT_ItemList" (.RowName (Utilities|Struct|BreakDataTableRowHandle (.ItemSelect (Utilities|Struct|BreakS_ItemSelect _array_element_2))))) (Utilities|Select :Index (.TypeItem (Utilities|Struct|BreakS_ItemSettings _returnvalue)) :NewEnumerator5 0 :NewEnumerator2 1 :NewEnumerator0 1 :NewEnumerator1 (Math|Random|RandomIntegerinRange 2 (.MaxAmount (Utilities|Struct|BreakS_ItemSettings _returnvalue))) :NewEnumerator3 (Math|Random|RandomIntegerinRange 100 (.MaxAmount (Utilities|Struct|BreakS_ItemSettings _returnvalue))) :NewEnumerator4 (Math|Random|RandomIntegerinRange 50 (.MaxAmount (Utilities|Struct|BreakS_ItemSettings _returnvalue))) :NewEnumerator7 1 :NewEnumerator8 1 :NewEnumerator6 1)))))))
    (for _index (range (.Minimum (Utilities|Struct|BreakS_typeItensRandomSpawn _array_element)) (Math|Random|RandomIntegerinRange (.Minimum (Utilities|Struct|BreakS_typeItensRandomSpawn _array_element)) (.Maximum (Utilities|Struct|BreakS_typeItensRandomSpawn _array_element))))
      (CallFunction|AddItensLootBox (Utilities|Array|Get(acopy) _itensspawn (Math|Random|RandomIntegerinRange 0 (- (Utilities|Array|Length _itensspawn) 1)))))
    (Utilities|Array|Clear (Variables|Default|GetItensSpawn))))

(fn GetAllItens
  (bind _outrownames (DataTable|GetDataTableRowNames "/Game/InventoryGrid/Blueprints/Modify_inventory/DT_ItemList.DT_ItemList"))
  (for _array_element _outrownames
    (if (Utilities|Name|NotEqual(Name) _array_element "empty")
      (Utilities|GetDataTableRow "/Game/InventoryGrid/Blueprints/Modify_inventory/DT_ItemList.DT_ItemList" _array_element
        (:then
          (Utilities|Array|Add (Variables|Default|GetAllItens) (Utilities|Struct|MakeS_ItemSelect (Utilities|Struct|MakeDataTableRowHandle "/Game/InventoryGrid/Blueprints/Modify_inventory/DT_ItemList.DT_ItemList" _array_element) 1))))))
  (return))