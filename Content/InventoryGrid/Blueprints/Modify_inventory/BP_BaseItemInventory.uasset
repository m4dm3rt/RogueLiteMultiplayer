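; BP_BaseItemInventory is a world item actor that can be picked up into an inventory component.
; Its data table row sets the static or skeletal mesh and the name widget.
; BeginPlay builds a BP_BaseItemobject if none is valid, storing a randomly chosen gun material on it.
; Pickup tries equipping, then auto-stacking, then adding to inventory, and destroys the actor on success.
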(event Custom|TryDestroyActor
  (params (Target :type Actor%20Object%20Reference))
  ;[0 0.5 0.01618] BeginPlay
  (Actor|DestroyActor Target))

(event EventShowNameItem
  (params (Show? :type Boolean))
  ;[0 0.5 0.01618] BeginPlay
  (Rendering|SetVisibility (Variables|Default|GetWidget) Show? false))

(event EventPickUpInteraction
  (params (InventoryComponent :type BP%20Inventory%20Grid%20Component%20Object%20Reference))
  ;[1 0 0] Try PickUP
  (bind _value (Default|AddItemtoEquipment InventoryComponent (Variables|Private|GetItem) "NewEnumerator2"))
  (if _value
    (CallFunction|TryDestroyActor self)
    (else
      (bind _success (Default|AutomaticStack InventoryComponent (Variables|Private|GetItem)))
      (if _success
        (CallFunction|TryDestroyActor self :!label _label)
        (else
          (bind _success_2 (Default|AddItemtoInventory InventoryComponent (Variables|Private|GetItem) false))
          (if _success_2
            (goto _label)))))))

(event EventBeginPlay
  (bind _itemselect (Variables|Default|GetItemSelect))
  (bind _skeletalmesh (Variables|Default|GetSkeletalMesh))
  (bind _itemselect_2 (Utilities|Struct|BreakS_ItemSelect _itemselect))
  (bind (_datatable _rowname) (Utilities|Struct|BreakDataTableRowHandle _itemselect_2))
  ;[0 0.5 0.01618] BeginPlay
  (Utilities|FlowControl|Sequence
    (:then_0
      (bind _returnvalue (Utilities|GetDataTableRow _datatable _rowname)
        (:then
          (Variables|Private|SetItem%20Settings _returnvalue)
          (if (not (Utilities|IsValid (Variables|Private|GetItem)))
            (bind _itemobject (CallFunction|GetDefaultItemObject))
            (bind _output_get (Variables|Private|SetItem _itemobject))
            (Rendering|Material|SetMaterial _skeletalmesh 0 (select (Math|Random|RandomBool) "/Game/InventoryGrid/Demo/FirstPerson/FPWeapon/Materials/M_FPGun_Inst1.M_FPGun_Inst1" "/Game/InventoryGrid/Demo/FirstPerson/FPWeapon/Materials/M_FPGun_Inst2.M_FPGun_Inst2"))
            (Default|SetMaterialCustom _output_get (Rendering|Material|GetMaterial _skeletalmesh 0))))))
    (:then_1
      (bind _aswb_name_item (Utilities|Casting|CastToWB_NameItem (UserInterface|GetUserWidgetObject (Variables|Default|GetWidget))))
      (bind _output_get_2 (Variables|Default|SetAs%20WB%20Name%20Item _aswb_name_item))
      (Variables|/Game/InventoryGrid/Blueprints/Widget/WB_NameItem.WB_NameItem_C|SetNameItem _output_get_2 (.Name (Utilities|Struct|BreakS_ItemSettings (Variables|Private|GetItem%20Settings)))))))

(fn ConstructionScript
  (bind _itemselect (Variables|Default|GetItemSelect))
  (bind _itemselect_2 (Utilities|Struct|BreakS_ItemSelect _itemselect))
  (bind (_datatable _rowname) (Utilities|Struct|BreakDataTableRowHandle _itemselect_2))
  (bind _returnvalue (Utilities|GetDataTableRow _datatable _rowname)
    (:then
      (Variables|Private|SetItem%20Settings _returnvalue)
      (if (== (.SkeletalMesh (Utilities|Struct|BreakS_ItemSettings _returnvalue)) 0)
        (Components|StaticMesh|SetStaticMesh (Variables|Default|GetStaticMesh) (.StaticMesh (Utilities|Struct|BreakS_ItemSettings _returnvalue)))
        (Rendering|SetVisibility (Variables|Default|GetSkeletalMesh) false false)
        (Transformation|AttachComponentToComponent (Variables|Default|GetWidget) (Variables|Default|GetStaticMesh) "None" "SnapToTarget" "SnapToTarget" "SnapToTarget" true)
        (if (== (Variables|/Script/Engine.StaticMeshComponent|GetStaticMesh (Variables|Default|GetStaticMesh)) "/Game/InventoryGrid/Blueprints/Map/Geometry/Meshes/SM_Cube.SM_Cube")
          (Transformation|SetWorldScale3D (Variables|Default|GetStaticMesh) "0.300000,0.300000,0.300000"))
        (else
          (Components|SkinnedMesh|SetSkinnedAssetandUpdate (Variables|Default|GetSkeletalMesh) (.SkeletalMesh (Utilities|Struct|BreakS_ItemSettings _returnvalue)) true)
          (Rendering|SetVisibility (Variables|Default|GetStaticMesh) false false)
          (Transformation|AttachComponentToComponent (Variables|Default|GetWidget) (Variables|Default|GetSkeletalMesh) "None" "SnapToTarget" "SnapToTarget" "SnapToTarget" true))))))

(fn GetDefaultItemObject
  (bind _returnvalue (Game|ConstructObjectfromClass self "/Game/InventoryGrid/Blueprints/Structs/BP_BaseItemobject.BP_BaseItemobject_C" (Utilities|GetClass self) (Variables|Private|GetItem%20Settings) (Variables|Default|GetItemSelect)))
  (Default|SetSettings _returnvalue)
  (Default|SetCurrentAmmo _returnvalue (Variables|Default|GetCurrentAmmoWeapon))
  (return _returnvalue))