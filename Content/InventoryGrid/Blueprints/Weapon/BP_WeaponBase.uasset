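; Base weapon Blueprint for an inventory-driven shooter, taking its settings and skeletal mesh from a data table row.
; Firing line-traces to apply random damage, show damage numbers and hit markers, and trigger recoil, camera shake and AI noise.
; Looping MultiGates cycle the permitted fire modes, with delayed re-entry driving burst and full-auto.
; Ammo count syncs to the linked item, and reloading removes "Ammo" from the player's inventory.
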(event Custom|Reload
  ;[0 0.6977 1] Reload Logic
  (if (not (Variables|Default|GetIs%20Reloading?))
    (|Logic_reload)))

(event Custom|modefire
  ;[0 1 0.811 1 50] ModeFire
  (if (not (Utilities|Enum|Equal(Enum) (Variables|ConfigWeapon|GetSwitch%20Firing%20Modes) "NewEnumerator0"))
    (if (not (Utilities|Enum|Equal(Enum) (Variables|ConfigWeapon|GetSwitch%20Firing%20Modes) "NewEnumerator1"))
      (if (not (Utilities|Enum|Equal(Enum) (Variables|ConfigWeapon|GetSwitch%20Firing%20Modes) "NewEnumerator2"))
        (if (Utilities|Enum|Equal(Enum) (Variables|ConfigWeapon|GetSwitch%20Firing%20Modes) "NewEnumerator3")
          (Utilities|FlowControl|MultiGate false true -1
            (:Out%200
              (Variables|Default|SetModeState "NewEnumerator1"))
            (:Out%201
              (Variables|Default|SetModeState "NewEnumerator0")))
          (elif (Utilities|Enum|Equal(Enum) (Variables|ConfigWeapon|GetSwitch%20Firing%20Modes) "NewEnumerator4")
            (Utilities|FlowControl|MultiGate false true -1
              (:Out%200
                (Variables|Default|SetModeState "NewEnumerator2"))
              (:Out%201
                (Variables|Default|SetModeState "NewEnumerator0")))
            (elif (Utilities|Enum|Equal(Enum) (Variables|ConfigWeapon|GetSwitch%20Firing%20Modes) "NewEnumerator5")
              (Utilities|FlowControl|MultiGate false true -1
                (:Out%200
                  (Variables|Default|SetModeState "NewEnumerator2"))
                (:Out%201
                  (Variables|Default|SetModeState "NewEnumerator1")))
              (elif (Utilities|Enum|Equal(Enum) (Variables|ConfigWeapon|GetSwitch%20Firing%20Modes) "NewEnumerator6")
                (Utilities|FlowControl|MultiGate false true -1
                  (:Out%200
                    (Variables|Default|SetModeState "NewEnumerator2"))
                  (:Out%201
                    (Variables|Default|SetModeState "NewEnumerator1"))
                  (:Out%202
                    (Variables|Default|SetModeState "NewEnumerator0")))))))))))

(event Custom|WeaponRecoil
  (params (Pitch :type Float%20%28double-precision%29) (Yaw :type Float%20%28double-precision%29))
  (bind _returnvalue (Game|GetPlayerCharacter 0))
  (bind _returnvalue_2 (* Yaw 1.0))
  ;[0.8716 1 0 1 50] Recoil System
  (Pawn|Input|AddControllerPitchInput _returnvalue (select false (/ (* Pitch 1.0) 2.0) Pitch))
  (Pawn|Input|AddControllerYawInput _returnvalue (select false (/ _returnvalue_2 2.0) _returnvalue_2)))

(event Custom|StartFire
  ;[1 0 0] Fire Logic
  (if (Variables|Default|GetIs%20Fire?)
    (|Logic_fire)))

(event EventBeginPlay
  (bind _item (Variables|Default|GetItem)
    (:then
      (bind _material_interface (Variables|/Game/InventoryGrid/Blueprints/Structs/BP_BaseItemobject.BP_BaseItemobject_C|GetMaterial%20Interface _item)
        (:then
          (Rendering|Material|SetMaterial (Variables|Default|GetSkeletalMesh) 0 _material_interface))
        (:else)))
    (:else)))

(fn ConstructionScript
  (bind _item_select (Variables|Default|GetItem%20Select))
  (bind _itemselect (Utilities|Struct|BreakS_ItemSelect _item_select))
  (bind (_datatable _rowname) (Utilities|Struct|BreakDataTableRowHandle _itemselect))
  ;[0 0 0] Set Skeletal Mesh Weapon
  (bind _returnvalue (Utilities|GetDataTableRow _datatable _rowname)
    (:then
      (Variables|Default|SetItemSettings _returnvalue)
      (Components|SkinnedMesh|SetSkinnedAssetandUpdate (Variables|Default|GetSkeletalMesh) (.SkeletalMesh (Utilities|Struct|BreakS_ItemSettings _returnvalue)) true))))

(fn SetAllAmmo
  (params (Set%20Allammo :type Integer))
  (Variables|Default|SetAll%20Ammo%20Inventory Set%20Allammo))

(fn SetCurrentAmmo
  (params (Item :type BP%20Base%20Itemobject%20Object%20Reference) (CurrentAmmo :type Integer))
  (bind _output_get (Variables|Default|SetItem_W Item))
  (Variables|Default|SetCurrentAmmo CurrentAmmo)
  (Variables|Default|SetClipSize (.ClipSizeWeapon (Utilities|Struct|BreakS_EquipementSettings (.EquipmentSettings (Utilities|Struct|BreakS_ItemSettings (Variables|/Game/InventoryGrid/Blueprints/Structs/BP_BaseItemobject.BP_BaseItemobject_C|GetItemSettings _output_get)))))))

(fn SetAmmoInventory
  (Default|SetCurrentAmmo (Variables|Default|GetItem) (Variables|Default|GetCurrentAmmo)))

(fn FloatingDamage
  (params (Damage :type Float%20%28double-precision%29) (Hit :type Hit%20Result%20Structure))
  (bind (_bblockinghit _binitialoverlap _time _distance _location _impactpoint _normal _impactnormal _physmat _hitactor) (Collision|BreakHitResult Hit))
  (if (> Damage 0.0)
    (if (or (Utilities|IsValid (.AsCharacter (Utilities|Casting|CastToCharacter _hitactor))) (Utilities|IsValid (.AsBP%20Target (Utilities|Casting|CastToBP_target _hitactor))))
      (Game|SpawnActorfromClass "/Game/InventoryGrid/Blueprints/Widget/FloatingDamage/BP_ActorFloating.BP_ActorFloating_C" (Math|Transform|MakeTransform _impactpoint "0, 0, 0" "1.000000,1.000000,1.000000") "Undefined" "OverrideRootScale" 0 (Utilities|Text|ToText(Integer) (Math|Float|Truncate Damage)) 0)
      (bind _inventory (Class|BPInventoryGridPlayer|Getinventory(Message) (Game|GetPlayerCharacter 0)))
      (bind _mainhud (Variables|/Game/InventoryGrid/Blueprints/Modify_inventory/BP_InventoryGridComponent.BP_InventoryGridComponent_C|GetMainHud _inventory)
        (:then
          (Default|HitEvent (Variables|/Game/InventoryGrid/Blueprints/Widget/WB_MainHud.WB_MainHud_C|GetWB_Hit_C_1 _mainhud)))
        (:else)))))

(fn Target
  (params (Target :type Actor%20Object%20Reference))
  (bind _asbp_target (Utilities|Casting|CastToBP_target Target))
  (Default|Hit _asbp_target))

(fn ContainerSpawn?
  (return false))

(event Custom|Burst%20Fire
  (if (> (Variables|Default|GetCurrentAmmo) 0)
    (Utilities|FlowControl|Delay 0.05)
    (return)
    (else
      (Variables|Default|SetIs%20Fire? false))))

(event Custom|Full%20Auto%20Fire
  (if (Variables|Default|GetIs%20Fire?)
    (if (> (Variables|Default|GetCurrentAmmo) 0)
      (Utilities|FlowControl|Delay (Variables|ConfigWeapon|GetFireRate))
      (return)
      (else
        (Variables|Default|SetIs%20Fire? false)))))

(event Custom|WeaponReload
  (Variables|Default|SetIs%20Reloading? false)
  (Variables|Default|SetNeeded%20Ammo (- (Variables|Default|GetClipSize) (Variables|Default|GetCurrentAmmo)))
  (if (<= (Variables|Default|GetAll%20Ammo%20Inventory) (Variables|Default|GetNeeded%20Ammo))
    (Variables|Default|SetCurrentAmmo (+ (Variables|Default|GetCurrentAmmo) (Variables|Default|GetAll%20Ammo%20Inventory)))
    (CallFunction|SetAmmoInventory)
    (else
      (Variables|Default|SetAll%20Ammo%20Inventory (- (Variables|Default|GetAll%20Ammo%20Inventory) (Variables|Default|GetNeeded%20Ammo)))
      (Variables|Default|SetCurrentAmmo (Variables|Default|GetClipSize))
      (CallFunction|SetAmmoInventory)))
  (bind _inventory (Class|BPInventoryGridPlayer|Getinventory(Message) (Game|GetPlayerCharacter 0)))
  (Default|RemoveItemName _inventory "Ammo" (Variables|Default|GetNeeded%20Ammo)))

(fn GetWeapon
  (return (Variables|Default|GetItemSettings)))

(fn GetWeaponActor
  (return self))