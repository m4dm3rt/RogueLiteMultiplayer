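; Base workbench actor for the inventory grid system that opens a crafting inventory on interaction and runs timed crafts.
; Interaction registers the bench with the player's InventoryComponent and toggles its workbench UI.
; A looping one-second timer counts down the recipe's craft time, then flags items as ready to collect.
; A box overlap shows or hides the bench's widget component UI, which is notified when crafting starts and stops.
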(event OnComponentBeginOverlap(Box)
  (params (OverlappedComponent :type Primitive%20Component%20Object%20Reference) (OtherActor :type Actor%20Object%20Reference) (OtherComp :type Primitive%20Component%20Object%20Reference) (OtherBodyIndex :type Integer) (bFromSweep :type Boolean) (SweepResult :type Hit%20Result%20Structure%20%28by%20ref%29))
  ;[1 0 0.2192] Show Widget WorkBench
  (if (== OtherActor (Game|GetPlayerCharacter 0))
    (bind _as_wb_work_bench (Variables|Default|GetAs%20WB%20Work%20Bench)
      (:then
        (Widget|SetVisibility _as_wb_work_bench "Visible"))
      (:else))))

(event OnComponentEndOverlap(Box)
  (params (OverlappedComponent :type Primitive%20Component%20Object%20Reference) (OtherActor :type Actor%20Object%20Reference) (OtherComp :type Primitive%20Component%20Object%20Reference) (OtherBodyIndex :type Integer))
  ;[1 0 0.2192] Show Widget WorkBench
  (if (== OtherActor (Game|GetPlayerCharacter 0))
    (bind _as_wb_work_bench (Variables|Default|GetAs%20WB%20Work%20Bench)
      (:then
        (Widget|SetVisibility _as_wb_work_bench "Hidden"))
      (:else))))

(event Custom|ExitLootBox
  ;[0 0.25 1] Open UI
  (Default|ToggleInventory (Variables|Default|GetInventory%20Component%20Player))
  (Variables|Default|SetOpen? false))

(event Custom|AddCraft
  (params (List :type S%20Work%20Bench%20Structure) (ID :type Integer))
  ;[0 0.5 0.01618] Row Craft
  (bind _output_get (Variables|Default|SetListCraft List))
  (Variables|Default|SetIDItemCraft ID)
  (Variables|Default|SetTime%20to%20Craft (.TimeToCraft (Utilities|Struct|BreakS_WorkBench _output_get)))
  (bind _returnvalue (Utilities|Time|SetTimerbyEvent (delegate Custom|DownTime) 1.0 true))
  (Variables|Default|SetEvent _returnvalue)
  (Variables|Default|SetIsCrafting? true)
  (Default|Start (Variables|Default|GetAs%20WB%20Work%20Bench) self))

(event Custom|DownTime
  ;[0 0.5 0.01618] Row Craft
  (bind _output_get (Variables|Default|SetTime%20to%20Craft (- (Variables|Default|GetTime%20to%20Craft) 1.0)))
  (if (< _output_get 0.0)
    (Variables|Default|SetIsCrafting? false)
    (Variables|Default|SetGetItens? true)
    (Utilities|Time|PauseTimerbyHandle (Variables|Default|GetEvent))
    (Default|Stop (Variables|Default|GetAs%20WB%20Work%20Bench))))

(event EventBeginPlay
  ;[0 0.5 0.01618] BeginPlay
  (bind _aswb_work_bench (Utilities|Casting|CastToWB_WorkBench (UserInterface|GetUserWidgetObject (Variables|Default|GetWidget))))
  (Variables|Default|SetAs%20WB%20Work%20Bench _aswb_work_bench))

(event EventStartInteraction
  (params (InventoryComponent :type BP%20Inventory%20Grid%20Component%20Object%20Reference))
  ;[0 0.25 1] Open UI
  (bind _output_get (Variables|Default|SetInventory%20Component%20Player InventoryComponent))
  (Variables|/Game/InventoryGrid/Blueprints/Modify_inventory/BP_InventoryGridComponent.BP_InventoryGridComponent_C|SetWorkBench _output_get self)
  (Variables|Default|SetOpen? (Widget|IsVisible (Variables|/Game/InventoryGrid/Blueprints/Modify_inventory/BP_InventoryGridComponent.BP_InventoryGridComponent_C|GetInventoryUI _output_get)))
  (if (Variables|Default|GetOpen?)
    (Default|ToggleInventory (Variables|Default|GetInventory%20Component%20Player))
    (Variables|Default|SetOpen? false)
    (else
      (Default|ToggleInventory (Variables|Default|GetInventory%20Component%20Player) "workbench")
      (Variables|Default|SetOpen? true))))

(fn ConstructionScript)