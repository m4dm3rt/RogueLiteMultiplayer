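; Base backpack actor for the grid inventory: a world pickup that carries its own item container.
; The construction script reads a DataTable row to set the mesh and grid size, and BeginPlay creates its item object and fills the name widget.
; Interaction tries equipping, then storing in inventory, destroying the actor on success, otherwise opens it as a loot box.
; Saved contents are restored from the item object into the grid component.
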(event EventStartInteraction
  (params (InventoryComponent :type BP%20Inventory%20Grid%20Component%20Object%20Reference))
  (bind _itemobject (Variables|Default|GetItemObject))
  ;[0 0.6117 1] PickUp
  (Variables|Default|SetInventory%20ComponentPlayer InventoryComponent)
  (CallFunction|SetInventoryBackPack)
  (if (Utilities|Enum|Equal(Enum) (Utilities|Struct|BreakS_ItemSettings (Variables|Default|GetItem%20Settings)) "NewEnumerator8")
    (bind _value (Default|AddItemtoEquipment InventoryComponent _itemobject "NewEnumerator2"))
    (if _value
      (Actor|DestroyActor)
      (else
        (bind _success (Default|AddItemtoInventory InventoryComponent _itemobject false))
        (if _success
          (Actor|DestroyActor)
          (else
            (Variables|/Game/InventoryGrid/Blueprints/Modify_inventory/BP_InventoryGridComponent.BP_InventoryGridComponent_C|SetBackPackContainer? (Variables|Default|GetBP_InventoryGridComponent) true)
            (Default|GetBackPackContainer (Variables|Default|GetInventory%20ComponentPlayer) self)
            (Default|ToggleInventory (Variables|Default|GetInventory%20ComponentPlayer) "LootBox")
            (CallFunction|CheckComponents (Variables|/Game/InventoryGrid/Blueprints/Modify_inventory/BP_InventoryGridComponent.BP_InventoryGridComponent_C|GetInventoryUI (Variables|Default|GetInventory%20ComponentPlayer)))))))))

(event EventBeginPlay
  ;[0 0.5 0.01618] BeginPlay
  (Utilities|FlowControl|Sequence
    (:then_0
      (if (not (Utilities|IsValid (Variables|Default|GetItemObject)))
        (bind _returnvalue (Game|ConstructObjectfromClass self "/Game/InventoryGrid/Blueprints/Structs/BP_BaseItemobject.BP_BaseItemobject_C" (Utilities|GetClass self) (Variables|Default|GetItem%20Settings) (Variables|Config|GetItemSelect)))
        (Default|SetSettings _returnvalue)
        (Variables|Default|SetItemObject _returnvalue)))
    (:then_1
      (bind _aswb_name_item (Utilities|Casting|CastToWB_NameItem (UserInterface|GetUserWidgetObject (Variables|Default|GetWidget))))
      (bind _output_get (Variables|Default|SetAs%20WB%20Name%20Item _aswb_name_item))
      (Variables|/Game/InventoryGrid/Blueprints/Widget/WB_NameItem.WB_NameItem_C|SetNameItem _output_get (Utilities|Struct|BreakS_ItemSettings (Variables|Default|GetItem%20Settings))))))

(event EventShowNameItem
  (params (Show? :type Boolean))
  ;[0 0.5 0.01618] BeginPlay
  (Rendering|SetVisibility (Variables|Default|GetWidget) Show? false))

(event EventSetContainer
  (params (Item :type BP%20Base%20Itemobject%20Object%20Reference))
  (bind _inventory (Default|GetInventory Item))
  ;[1 0 0] Get Or set Inventory Array
  (Variables|Default|SetItemObject Item)
  (if (> (Utilities|Array|Length _inventory) 0)
    (Variables|/Game/InventoryGrid/Blueprints/Modify_inventory/BP_InventoryGridComponent.BP_InventoryGridComponent_C|SetInventory (Variables|Default|GetBP_InventoryGridComponent) _inventory)))

(event EventSetInventory
  (params (Inventory :type BP%20Inventory%20Grid%20Component%20Object%20Reference) (Item :type BP%20Base%20Itemobject%20Object%20Reference))
  (bind _inventory (Default|GetInventory Item))
  ;[1 0 0] Get Or set Inventory Array
  (Variables|/Game/InventoryGrid/Blueprints/Modify_inventory/BP_InventoryGridComponent.BP_InventoryGridComponent_C|SetBackPack Inventory self)
  (Variables|/Game/InventoryGrid/Blueprints/Modify_inventory/BP_InventoryGridComponent.BP_InventoryGridComponent_C|SetInventoryPlayer (Variables|Default|GetBP_InventoryGridComponent) Inventory)
  (if (> (Utilities|Array|Length _inventory) 0)
    (Variables|/Game/InventoryGrid/Blueprints/Modify_inventory/BP_InventoryGridComponent.BP_InventoryGridComponent_C|SetInventory (Variables|Default|GetBP_InventoryGridComponent) _inventory)))

(fn ConstructionScript
  (bind _bp_inventorygridcomponent (Variables|Default|GetBP_InventoryGridComponent))
  (bind _itemselect (Variables|Config|GetItemSelect))
  (bind _itemselect_2 (Utilities|Struct|BreakS_ItemSelect _itemselect))
  (bind (_datatable _rowname) (Utilities|Struct|BreakDataTableRowHandle _itemselect_2))
  (bind _returnvalue (Utilities|GetDataTableRow _datatable _rowname)
    (:then
      (Variables|Default|SetItem%20Settings _returnvalue)
      (Components|SkinnedMesh|SetSkinnedAssetandUpdate (Variables|Default|GetSkeletalMesh) (.SkeletalMesh (Utilities|Struct|BreakS_ItemSettings (Variables|Default|GetItem%20Settings))) true)
      (Variables|/Game/InventoryGrid/Blueprints/Modify_inventory/BP_InventoryGridComponent.BP_InventoryGridComponent_C|SetColumns _bp_inventorygridcomponent (.Columns (Utilities|Struct|BreakS_ContainerConfig (.ContainerSettings (Utilities|Struct|BreakS_ItemSettings (Variables|Default|GetItem%20Settings))))))
      (Variables|/Game/InventoryGrid/Blueprints/Modify_inventory/BP_InventoryGridComponent.BP_InventoryGridComponent_C|SetRows _bp_inventorygridcomponent (.Rows (Utilities|Struct|BreakS_ContainerConfig (.ContainerSettings (Utilities|Struct|BreakS_ItemSettings (Variables|Default|GetItem%20Settings)))))))))

(fn CheckComponents
  (params (InventoryUI :type WB%20Inventory%20Object%20Reference))
  (Default|GetInventorySettings (Variables|/Game/InventoryGrid/Blueprints/Widget/WB_LootBoxPanel.WB_LootBoxPanel_C|GetWB_GridPanelInventoryLootBox (Variables|/Game/InventoryGrid/Blueprints/Widget/WB_Inventory.WB_Inventory_C|GetWB_LootBox InventoryUI)) InventoryUI (Variables|Default|GetBP_InventoryGridComponent) (Variables|Default|GetInventory%20ComponentPlayer) 0 0 "" "NewEnumerator5" false)
  (Default|Name (Variables|/Game/InventoryGrid/Blueprints/Widget/WB_Inventory.WB_Inventory_C|GetWB_LootBox (Variables|/Game/InventoryGrid/Blueprints/Modify_inventory/BP_InventoryGridComponent.BP_InventoryGridComponent_C|GetInventoryUI (Variables|Default|GetInventory%20ComponentPlayer))) (Utilities|Text|ToText(String) (Utilities|Struct|BreakS_ItemSettings (Variables|Default|GetItem%20Settings)))))

(fn SetInventoryBackPack
  (bind _itemobject (Variables|Default|GetItemObject))
  (bind _inventory (Default|GetInventory _itemobject))
  (if (> (Utilities|Array|Length _inventory) 0)
    (Variables|/Game/InventoryGrid/Blueprints/Modify_inventory/BP_InventoryGridComponent.BP_InventoryGridComponent_C|SetInventory (Variables|Default|GetBP_InventoryGridComponent) _inventory)))

(fn ContainerSpawn?
  (return false))

(fn GetWeapon
  (return ""))

(fn GetWeaponActor
  (return 0))