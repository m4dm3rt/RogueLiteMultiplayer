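; Base actor for a tactical rig: a world pickup that equips into the player's inventory and provides its own storage grid.
; The construction script pulls settings from a data table row to set the skeletal mesh and grid dimensions.
; BeginPlay creates an item object if none exists; interaction adds it to equipment and destroys the actor on success.
; SetInventory links the rig to the player inventory and restores any contents saved on the item.
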(event EventBeginPlay
  ;[0 0.5 0.01618] BeginPlay
  (if (not (Utilities|IsValid (Variables|Default|GetItemObject)))
    (bind _returnvalue (Game|ConstructObjectfromClass self "/Game/InventoryGrid/Blueprints/Structs/BP_BaseItemobject.BP_BaseItemobject_C" (Utilities|GetClass self) (Variables|Default|GetItem%20Settings) (Variables|Default|GetItemSelect)))
    (Default|SetSettings _returnvalue)
    (Variables|Default|SetItemObject _returnvalue)))

(event EventStartInteraction
  (params (InventoryComponent :type BP%20Inventory%20Grid%20Component%20Object%20Reference))
  ;[0 0.5 0.01618] PickUp
  (bind _value (Default|AddItemtoEquipment InventoryComponent (Variables|Default|GetItemObject) "NewEnumerator2"))
  (if _value
    (Actor|DestroyActor)))

(event EventSetInventory
  (params (Inventory :type BP%20Inventory%20Grid%20Component%20Object%20Reference) (Item :type BP%20Base%20Itemobject%20Object%20Reference))
  (bind _inventory (Default|GetInventory Item))
  ;[1 0 0] Set inventory Array
  (Variables|/Game/InventoryGrid/Blueprints/Modify_inventory/BP_InventoryGridComponent.BP_InventoryGridComponent_C|SetTacticalRig Inventory self)
  (Variables|/Game/InventoryGrid/Blueprints/Modify_inventory/BP_InventoryGridComponent.BP_InventoryGridComponent_C|SetInventoryPlayer (Variables|Default|GetBP_InventoryGridComponent) Inventory)
  (if (> (Utilities|Array|Length _inventory) 0)
    (Variables|/Game/InventoryGrid/Blueprints/Modify_inventory/BP_InventoryGridComponent.BP_InventoryGridComponent_C|SetInventory (Variables|Default|GetBP_InventoryGridComponent) _inventory)))

(fn ConstructionScript
  (bind _bp_inventorygridcomponent (Variables|Default|GetBP_InventoryGridComponent))
  (bind _itemselect (Variables|Default|GetItemSelect))
  (bind _itemselect_2 (Utilities|Struct|BreakS_ItemSelect _itemselect))
  (bind (_datatable _rowname) (Utilities|Struct|BreakDataTableRowHandle _itemselect_2))
  (bind _returnvalue (Utilities|GetDataTableRow _datatable _rowname)
    (:then
      (Variables|Default|SetItem%20Settings _returnvalue)
      (Components|SkinnedMesh|SetSkinnedAssetandUpdate (Variables|Default|GetSkeletalMesh) (.SkeletalMesh (Utilities|Struct|BreakS_ItemSettings (Variables|Default|GetItem%20Settings))) true)
      (Variables|/Game/InventoryGrid/Blueprints/Modify_inventory/BP_InventoryGridComponent.BP_InventoryGridComponent_C|SetColumns _bp_inventorygridcomponent (.Columns (Utilities|Struct|BreakS_ContainerConfig (.ContainerSettings (Utilities|Struct|BreakS_ItemSettings (Variables|Default|GetItem%20Settings))))))
      (Variables|/Game/InventoryGrid/Blueprints/Modify_inventory/BP_InventoryGridComponent.BP_InventoryGridComponent_C|SetRows _bp_inventorygridcomponent (.Rows (Utilities|Struct|BreakS_ContainerConfig (.ContainerSettings (Utilities|Struct|BreakS_ItemSettings (Variables|Default|GetItem%20Settings)))))))))

(fn ContainerSpawn?
  (return false))

(fn GetWeapon
  (return ""))

(fn GetWeaponActor
  (return 0))