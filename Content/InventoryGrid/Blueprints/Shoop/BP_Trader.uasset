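; BP_Trader is an interactable shop actor for the grid inventory system.
; On BeginPlay it stocks its Buy inventory from either all DT_ItemList rows or ItensForSale, using spawned item actors that are destroyed once added.
; Interaction toggles the player's trader UI, while Buy and Sell bind the panel's grid to their respective inventory components.
; A box overlap shows or hides the trade icon widget for the player.
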(event OnComponentBeginOverlap(Box)
  (params (OverlappedComponent :type Primitive%20Component%20Object%20Reference) (OtherActor :type Actor%20Object%20Reference) (OtherComp :type Primitive%20Component%20Object%20Reference) (OtherBodyIndex :type Integer) (bFromSweep :type Boolean) (SweepResult :type Hit%20Result%20Structure%20%28by%20ref%29))
  ;[1 0 0] Visibility Icon Trade
  (if (== OtherActor (Game|GetPlayerCharacter 0))
    (bind _as_wb_trader (Variables|Default|GetAs%20WB%20Trader)
      (:then
        (Widget|SetVisibility _as_wb_trader "Visible"))
      (:else))))

(event OnComponentEndOverlap(Box)
  (params (OverlappedComponent :type Primitive%20Component%20Object%20Reference) (OtherActor :type Actor%20Object%20Reference) (OtherComp :type Primitive%20Component%20Object%20Reference) (OtherBodyIndex :type Integer))
  ;[1 0 0] Visibility Icon Trade
  (if (== OtherActor (Game|GetPlayerCharacter 0))
    (bind _as_wb_trader (Variables|Default|GetAs%20WB%20Trader)
      (:then
        (Widget|SetVisibility _as_wb_trader "Hidden"))
      (:else))))

(event Custom|ExitLootBox
  ;[0 0.5 0.01618] Open UI
  (Default|ToggleInventory (Variables|Default|GetInventory%20Component%20Player))
  (Variables|Default|SetOpen? false))

(event Custom|Sell
  (bind _inventory_component_player (Variables|Default|GetInventory%20Component%20Player))
  (bind _inventoryui (Variables|/Game/InventoryGrid/Blueprints/Modify_inventory/BP_InventoryGridComponent.BP_InventoryGridComponent_C|GetInventoryUI _inventory_component_player))
  ;[0 0 0] Event Sell
  (Utilities|IsValid (Variables|/Game/InventoryGrid/Blueprints/Modify_inventory/BP_InventoryGridComponent.BP_InventoryGridComponent_C|GetBackPack (Variables|Default|GetInventory%20Component%20Player))
    (:Is%20Valid
      (Default|GetInventorySettings (Variables|/Game/InventoryGrid/Blueprints/Widget/WB_TraderPanel.WB_TraderPanel_C|GetWB_GridPanelInventoryLootBox (Variables|/Game/InventoryGrid/Blueprints/Widget/WB_Inventory.WB_Inventory_C|GetWB_TraderPanel _inventoryui)) (Variables|/Game/InventoryGrid/Blueprints/Modify_inventory/BP_InventoryGridComponent.BP_InventoryGridComponent_C|GetInventoryUI (Variables|Default|GetInventory%20Component%20Player)) (Variables|Default|GetBP_InventorySystemComponentSell) (Variables|Default|GetInventory%20Component%20Player) 0 0 "" "NewEnumerator5" false))
    (:Is%20Not%20Valid
      (Default|GetInventorySettings (Variables|/Game/InventoryGrid/Blueprints/Widget/WB_TraderPanel.WB_TraderPanel_C|GetWB_GridPanelInventoryLootBox (Variables|/Game/InventoryGrid/Blueprints/Widget/WB_Inventory.WB_Inventory_C|GetWB_TraderPanel _inventoryui)) _inventoryui (Variables|Default|GetBP_InventorySystemComponentSell) (Variables|Default|GetInventory%20Component%20Player) 0 0 "" "NewEnumerator5" false))))

(event EventStartInteraction
  (params (InventoryComponent :type BP%20Inventory%20Grid%20Component%20Object%20Reference))
  ;[0 0.5 0.01618] Open UI
  (bind _output_get (Variables|Default|SetInventory%20Component%20Player InventoryComponent))
  (Variables|/Game/InventoryGrid/Blueprints/Modify_inventory/BP_InventoryGridComponent.BP_InventoryGridComponent_C|SetTrader _output_get self)
  (Variables|Default|SetOpen? (Widget|IsVisible (Variables|/Game/InventoryGrid/Blueprints/Modify_inventory/BP_InventoryGridComponent.BP_InventoryGridComponent_C|GetInventoryUI _output_get)))
  (if (Variables|Default|GetOpen?)
    (Default|ToggleInventory (Variables|Default|GetInventory%20Component%20Player))
    (Variables|Default|SetOpen? false)
    (else
      (Default|ToggleInventory (Variables|Default|GetInventory%20Component%20Player) "Trader")
      (CallFunction|Buy)
      (Variables|Default|SetOpen? true))))

(event EventBeginPlay
  ;[0 0.5 0.01618] begin Play
  (bind _aswb_trader (Utilities|Casting|CastToWB_Trader (UserInterface|GetUserWidgetObject (Variables|Default|GetWidget))))
  (Variables|Default|SetAs%20WB%20Trader _aswb_trader)
  ;[1 0 0] Itens Sell Shope
  (if (Variables|Default|GetSale%20All%20Itens%20Data%20Base?)
    (CallFunction|GetAllItens)
    (for _array_element (Variables|Default|GetAllItens)
      (CallFunction|SpawnItens _array_element))
    (else
      (for _array_element_2 (Variables|Default|GetItens%20For%20Sale)
        (CallFunction|SpawnItens _array_element_2)))))

(fn ConstructionScript)

(fn Buy
  (LocalVariables|SetUI (Variables|/Game/InventoryGrid/Blueprints/Modify_inventory/BP_InventoryGridComponent.BP_InventoryGridComponent_C|GetInventoryUI (Variables|Default|GetInventory%20Component%20Player)))
  (Utilities|IsValid (Variables|/Game/InventoryGrid/Blueprints/Modify_inventory/BP_InventoryGridComponent.BP_InventoryGridComponent_C|GetBackPack (Variables|Default|GetInventory%20Component%20Player))
    (:Is%20Valid
      (Default|GetInventorySettings (Variables|/Game/InventoryGrid/Blueprints/Widget/WB_TraderPanel.WB_TraderPanel_C|GetWB_GridPanelInventoryLootBox (Variables|/Game/InventoryGrid/Blueprints/Widget/WB_Inventory.WB_Inventory_C|GetWB_TraderPanel (LocalVariables|GetUI))) (LocalVariables|GetUI) (Variables|Default|GetBP_InventorySystemComponentBuy) (Variables|Default|GetInventory%20Component%20Player) 0 0 "" "NewEnumerator5" false))
    (:Is%20Not%20Valid
      (Default|GetInventorySettings (Variables|/Game/InventoryGrid/Blueprints/Widget/WB_TraderPanel.WB_TraderPanel_C|GetWB_GridPanelInventoryLootBox (Variables|/Game/InventoryGrid/Blueprints/Widget/WB_Inventory.WB_Inventory_C|GetWB_TraderPanel (LocalVariables|GetUI))) (LocalVariables|GetUI) (Variables|Default|GetBP_InventorySystemComponentBuy) (Variables|Default|GetInventory%20Component%20Player) 0 0 "" "NewEnumerator5" false)))
  (Default|Name (Variables|/Game/InventoryGrid/Blueprints/Widget/WB_Inventory.WB_Inventory_C|GetWB_TraderPanel (Variables|/Game/InventoryGrid/Blueprints/Modify_inventory/BP_InventoryGridComponent.BP_InventoryGridComponent_C|GetInventoryUI (Variables|Default|GetInventory%20Component%20Player))) (Variables|Default|GetName)))

(fn SpawnItens
  (params (Item%20Select :type S%20Item%20Select%20Structure))
  (bind _returnvalue (Game|SpawnActorfromClass "/Game/InventoryGrid/Blueprints/Modify_inventory/BP_BaseItemInventory.BP_BaseItemInventory_C" (Math|Transform|MakeTransform "0, 0, 0" "0, 0, 0" "1.000000,1.000000,1.000000") "Undefined" "OverrideRootScale" 0 0 Item%20Select 0 0))
  (bind _itemobject (Default|GetDefaultItemObject _returnvalue))
  (bind _success (Default|AddItemtoInventory (Variables|Default|GetBP_InventorySystemComponentBuy) _itemobject false))
  (if _success
    (Actor|DestroyActor _returnvalue)))

(fn GetAllItens
  (bind _outrownames (DataTable|GetDataTableRowNames "/Game/InventoryGrid/Blueprints/Modify_inventory/DT_ItemList.DT_ItemList"))
  (for _array_element _outrownames
    (if (Utilities|Name|NotEqual(Name) _array_element "empty")
      (Utilities|GetDataTableRow "/Game/InventoryGrid/Blueprints/Modify_inventory/DT_ItemList.DT_ItemList" _array_element
        (:then
          (Utilities|Array|Add (Variables|Default|GetAllItens) (Utilities|Struct|MakeS_ItemSelect (Utilities|Struct|MakeDataTableRowHandle "/Game/InventoryGrid/Blueprints/Modify_inventory/DT_ItemList.DT_ItemList" _array_element) 1))))))
  (return))