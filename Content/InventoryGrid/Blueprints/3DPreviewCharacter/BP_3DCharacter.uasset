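; BP_3DCharacter is a modular character for the inventory grid's 3D preview.
; The construction script makes Legs, Gloves, Boots and Torso follow MainMesh's pose through Leader Pose.
; BeginPlay maps headset, eyewear, helmet, gloves, armor and boots slots to their components, with MainMesh as helmet, and records their starting meshes as defaults.
; Rotate yaws MainMesh by the input vector's X to turn the preview.
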(event EventBeginPlay
  ;[0 0.5 0.01618 1 30] BeginPlay - Set mesh Modular
  (Variables|Default|SetModularMesh (Utilities|Struct|MakeS_GetModularSkeletalMesh "NewEnumerator1" (Variables|Default|GetHeadSet) (Variables|Default|GetEyewear) (Variables|Default|GetMainMesh) (Variables|Default|GetGloves) (Variables|Default|GetTorso) (Variables|Default|GetBoots)))
  (Variables|Default|SetDefault%20Modular%20Mesh (Utilities|Struct|MakeS_DefaultModularSkeletalMesh "NewEnumerator1" (Variables|/Script/Engine.SkeletalMeshComponent|GetSkeletalMeshAsset (Variables|Default|GetHeadSet)) (Variables|/Script/Engine.SkeletalMeshComponent|GetSkeletalMeshAsset (Variables|Default|GetEyewear)) (Variables|/Script/Engine.SkeletalMeshComponent|GetSkeletalMeshAsset (Variables|Default|GetMainMesh)) (Variables|/Script/Engine.SkeletalMeshComponent|GetSkeletalMeshAsset (Variables|Default|GetGloves)) (Variables|/Script/Engine.SkeletalMeshComponent|GetSkeletalMeshAsset (Variables|Default|GetTorso)) (Variables|/Script/Engine.SkeletalMeshComponent|GetSkeletalMeshAsset (Variables|Default|GetBoots)))))

(fn ConstructionScript
  (Components|SkinnedMesh|SetLeaderPoseComponent (Variables|Default|GetLegs) (Variables|Default|GetMainMesh) false false))

(fn Rotate
  (params (InVec :type Vector%202D%20Structure))
  (Transformation|AddLocalRotation (Variables|Default|GetMainMesh) (Math|Rotator|MakeRotator 0.0 0.0 (.X (Math|Vector2D|BreakVector2D InVec))) false false))