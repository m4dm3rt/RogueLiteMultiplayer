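; Base item object for the grid inventory, holding one item's data and runtime state behind getters and setters.
; SetSettings copies ItemSettings into working fields like size, icon, stacking, equipment and container inventory, taking the amount from ItemSelect.
; Rotation is a flag that swaps the reported grid dimensions; GetRotateOrigin restores the state saved by SetRotateOrigin.
; It also tracks ammo, armor points, ID and inventory open state.
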(event Custom|SetMaterialCustom
  (params (Material%20Interface :type Material%20Interface%20Object%20Reference))
  (Variables|Default|SetMaterial%20Interface Material%20Interface))

(event Custom|SetSettings
  (bind _itemsettings (Variables|Default|GetItemSettings))
  (bind (_typeitem _name _description _skeletalmesh _staticmesh _actortoeventeuse _dimension _dimensioniconequipments _icon _colorbackground _isstack_ _maxamount _weight _salevalue _purchaseprice _equipmentsettings _containersettings) (Utilities|Struct|BreakS_ItemSettings _itemsettings))
  (bind (_spawnactorweapon _spawnactor _armorpoint) (Utilities|Struct|BreakS_EquipementSettings _equipmentsettings))
  (Variables|Default|SetName _name)
  (Variables|Default|SetDimension (Utilities|Struct|MakeIntPoint (Math|Float|Truncate (.x _dimension)) (Math|Float|Truncate (.y _dimension))))
  (Variables|Default|SetIcon _icon)
  (Variables|Default|SetIs%20Stack _isstack_)
  (Variables|Default|SetAmount (Utilities|Struct|BreakS_ItemSelect (Variables|Default|GetItemSelect)))
  (Variables|Default|SetMaxAmount _maxamount)
  (Variables|Default|SetBase%20Equipment _spawnactor)
  (Variables|Default|SetColor _colorbackground)
  (Variables|Default|SetInventory (Utilities|Struct|BreakS_ContainerConfig _containersettings))
  (Variables|Default|SetArmor%20Point _armorpoint))

(fn GetItemDimension
  (bind _dimension (Variables|Default|GetDimension))
  (if (Variables|Default|GetIsRotate?)
    (return (Utilities|Struct|MakeIntPoint (.y _dimension) (.x _dimension)))
    (else
      (return (Variables|Default|GetDimension)))))

(fn GetItemIcon
  (return (Variables|Default|GetIcon)))

(fn GetItemClass
  (return (Variables|Default|GetItemClass)))

(fn Rotate
  (Variables|Default|SetIsRotate? (not (Variables|Default|GetIsRotate?))))

(fn IsRotateIcon?
  (return (Variables|Default|GetIsRotate?)))

(fn GetIsStack?
  (return (Variables|Default|GetIs%20Stack)))

(fn SetAmount
  (params (Amount :type Integer))
  (bind _output_get (Variables|Default|SetAmount Amount))
  (Variables|Default|SetItemSelect (Utilities|Struct|MakeS_ItemSelect (.ItemSelect (Utilities|Struct|BreakS_ItemSelect (Variables|Default|GetItemSelect))) _output_get))
  (return))

(fn GetAmount
  (return (Variables|Default|GetAmount)))

(fn GetMaxAmount
  (return (Variables|Default|GetMaxAmount)))

(fn GetItemSettings
  (return (Variables|Default|GetItemSettings)))

(fn GetEquipment
  (return (Variables|Default|GetBase%20Equipment)))

(fn GetItemSelect
  (return (Variables|Default|GetItemSelect)))

(fn GetColorBackGround
  (return (Variables|Default|GetColor)))

(fn SetInventory
  (params (Inventory :type Array%20of%20BP%20Base%20Itemobject%20Object%20References))
  (Variables|Default|SetInventory Inventory)
  (return))

(fn GetInventory
  (return (Variables|Default|GetInventory)))

(fn SetInventoryOpen
  (params (Open? :type Boolean))
  (Variables|Default|SetOpen? Open?)
  (return))

(fn GetInventoryOpen
  (return (Variables|Default|GetOpen?)))

(fn SetCurrentAmmo
  (params (Amount :type Integer))
  (Variables|Default|SetCurrentAmmo Amount)
  (return))

(fn SetArmorPoint
  (params (Point :type Integer))
  (Variables|Default|SetArmor%20Point Point)
  (return))

(fn GetArmorPoint
  (return (Variables|Default|GetArmor%20Point)))

(fn SetID
  (params (ID :type Array%20of%20Integers))
  (Variables|Default|SetID ID)
  (return))

(fn GetID
  (return (Variables|Default|GetID)))

(fn GetItemName
  (return (Variables|Default|GetName)))

(fn SetRotateOrigin
  (Variables|Default|SetRotateOrigin (Variables|Default|GetIsRotate?)))

(fn GetRotateOrigin
  (Variables|Default|SetIsRotate? (Variables|Default|GetRotateOrigin)))