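; BP_CorpseExample is a lootable ragdoll corpse with a modular skeletal body and its own grid inventory component.
; Construction makes the body-part meshes follow the main mesh's pose; BeginPlay registers them with the inventory component, enables physics and seeds sample gear items.
; StartInteraction toggles the interacting player's inventory UI and passes it the corpse inventory as the other container, while ExitLootBox toggles it closed.
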(event Custom|ExitLootBox
  ;[1 0 0] Open UI Corpse
  (Default|ToggleInventory (stale EventStartInteraction InventoryComponent))
  (Variables|Default|SetOpen? false))

(event EventBeginPlay
  (bind _bp_inventorysystemcomponent (Variables|Default|GetBP_InventorySystemComponent))
  ;[0 0.5 0.01618] get modular Mesh
  (Default|GetModularSkeletalMesh (Variables|Default|GetBP_InventorySystemComponent) "NewEnumerator1" (Variables|Default|GetHeadset) (Variables|Default|GetEyewear) (Variables|Character|GetMesh) (Variables|Default|GetGloves) (Variables|Default|GetTorso) (Variables|Default|GetBoots))
  (Physics|SetSimulatePhysics (Variables|Character|GetMesh) true)
  ;[0 0.5 0.01618] Add Item Inventory Corpse
  (Default|SelectAddItemtoInventory _bp_inventorysystemcomponent "Boots")
  (Default|SelectAddItemtoInventory _bp_inventorysystemcomponent "BackPackOrange")
  (Default|SelectAddItemtoInventory _bp_inventorysystemcomponent "tacticalrig")
  (Default|SelectAddItemtoInventory _bp_inventorysystemcomponent "BodyArmor"))

(event EventStartInteraction
  (params (InventoryComponent :type BP%20Inventory%20Grid%20Component%20Object%20Reference))
  ;[1 0 0] Open UI Corpse
  (Variables|Default|SetOpen? (Widget|IsVisible (Variables|/Game/InventoryGrid/Blueprints/Modify_inventory/BP_InventoryGridComponent.BP_InventoryGridComponent_C|GetInventoryUI InventoryComponent)))
  (if (Variables|Default|GetOpen?)
    (Default|ToggleInventory InventoryComponent)
    (Variables|Default|SetOpen? false)
    (else
      (Default|ToggleInventory InventoryComponent)
      (Class|BPInterfaceWIdget|GiveWidgetVariables(Message) (Variables|/Game/InventoryGrid/Blueprints/Modify_inventory/BP_InventoryGridComponent.BP_InventoryGridComponent_C|GetInventoryUI InventoryComponent) "Corpse Inventory" (Variables|Default|GetBP_InventorySystemComponent))
      (Variables|Default|SetOpen? true))))

(fn ConstructionScript
  (Components|SkinnedMesh|SetLeaderPoseComponent (Variables|Default|GetBoots) (Variables|Character|GetMesh) false false))